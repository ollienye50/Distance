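; Phone actor that opens a Phone_UI screen while something overlaps its Phone component.
; Begin overlap creates a new widget, adds it to the viewport, then enables mouse cursor and click events if the player pawn is BP_ThirdPersonCharacter.
; End overlap removes top-level Phone_UI widgets and disables both, after the same pawn check.
; Neither event checks which actor overlapped.
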(event OnComponentBeginOverlap(Phone)
  (params (OverlappedComponent :type Primitive%20Component%20Object%20Reference) (OtherActor :type Actor%20Object%20Reference) (OtherComp :type Primitive%20Component%20Object%20Reference) (OtherBodyIndex :type Integer) (bFromSweep :type Boolean) (SweepResult :type Hit%20Result%20Structure%20%28by%20ref%29))
  (bind _returnvalue (Game|GetPlayerController 0))
  (Development|PrintString "Open phone")
  (bind _returnvalue_2 (UserInterface|CreateWidget "/Game/Assets/Blueprints/Phone_UI.Phone_UI_C"))
  (UserInterface|Viewport|AddtoViewport _returnvalue_2 0)
  (Utilities|Casting|CastToBP_ThirdPersonCharacter (Game|GetPlayerCharacter 0))
  (Variables|/Script/Engine.PlayerController|SetbEnableClickEvents _returnvalue true)
  (Variables|/Script/Engine.PlayerController|SetbShowMouseCursor _returnvalue true))

(event OnComponentEndOverlap(Phone)
  (params (OverlappedComponent :type Primitive%20Component%20Object%20Reference) (OtherActor :type Actor%20Object%20Reference) (OtherComp :type Primitive%20Component%20Object%20Reference) (OtherBodyIndex :type Integer))
  (bind _returnvalue (Game|GetPlayerController 0))
  (Development|PrintString "Close phone")
  (Utilities|Casting|CastToBP_ThirdPersonCharacter (Game|GetPlayerCharacter 0))
  (bind _foundwidgets (Widget|GetAllWidgetsOfClass "/Game/Assets/Blueprints/Phone_UI.Phone_UI_C" true))
  (Widget|RemovefromParent _foundwidgets)
  (Variables|/Script/Engine.PlayerController|SetbEnableClickEvents _returnvalue false)
  (Variables|/Script/Engine.PlayerController|SetbShowMouseCursor _returnvalue false))

(event EventBeginPlay)

(event Collision|EventActorBeginOverlap
  (params (OtherActor :type Actor%20Object%20Reference)))

(event EventTick
  (params (DeltaSeconds :type Float%20%28single-precision%29)))

(fn ConstructionScript)